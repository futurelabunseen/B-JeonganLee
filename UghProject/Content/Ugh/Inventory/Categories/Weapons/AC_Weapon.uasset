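; AC_Weapon is a weapon inventory component that grants weapons by name into a Weapons map.
; Give looks up the name in WeaponTable and exits if no row matches.
; A new weapon is added with its row data.
; For an owned weapon, it sets Ammo on the Find result to the table value, without summing or re-adding it to the map.
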(fn Give
  (params (WeaponName :type Name))
  (bind _weapons (Variables|Default|GetWeapons))
  (bind (_value _returnvalue) (Utilities|Map|Find _weapons WeaponName))
  (Utilities|FlowControl|Sequence
    (:then_0
      ;[1 1 1] Vaildate
      (bind _returnvalue_2 (Utilities|GetDataTableRow "/Game/Ugh/Inventory/Categories/Weapons/WeaponTable.WeaponTable" WeaponName)
        (:then
          (Variables|Default|SetOut%20Row _returnvalue_2))
        (:RowNotFound
          (Variables|Default|SetOut%20Row "")
          (return))))
    (:then_1
      ;[1 1 1] Stack
      (if _returnvalue
        (Utilities|Struct|SetmembersinWeaponStruct _value (Utilities|Struct|BreakWeaponStruct (Variables|Default|GetOut%20Row)))
        (return)))
    (:then_2
      ;[1 1 1] Add
      (Utilities|Map|Add (Variables|Default|GetWeapons) WeaponName (Variables|Default|GetOut%20Row))
      (return))))